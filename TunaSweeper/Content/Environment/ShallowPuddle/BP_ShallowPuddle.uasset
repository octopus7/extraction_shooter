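; BP_ShallowPuddle is a shallow puddle actor that shows a Niagara effect when footsteps land on it.
; On BeginPlay it binds to the OnPuddleFootstep event, which supplies the surface location and sprint state.
; Outside dedicated servers, each step spawns an inactive system just above the surface, sets its step strength higher for sprinting, then activates it.
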(event `self.ReceiveBeginPlay`
  (`parent.ReceiveBeginPlay`)
  (add `self.OnPuddleFootstep` (delegate `HandlePuddleFootstep`)))

(event `HandlePuddleFootstep` :!signature `self.OnPuddleFootstep`
  (params (SurfaceLocation :type "Vector Structure") (SpeedCmPerSecond :type "Float (single-precision)") (bSprinting :type Boolean) (StepInstigator :type "Actor Object Reference"))
  (if (not (`KismetSystemLibrary.IsDedicatedServer`))
    (bind _returnvalue (`NiagaraFunctionLibrary.SpawnSystemAtLocation` "/Game/Environment/ShallowPuddle/FX/NS_ShallowPuddle_Footstep.NS_ShallowPuddle_Footstep" (+ SurfaceLocation (0.0 0.0 0.3)) (struct) (1.0 1.0 1.0) true false))
    (`/Engine/EditorBlueprintResources/StandardMacros.IsValid` _returnvalue
      (:`Is Valid`
        (`NiagaraComponent.SetVariableFloat` _returnvalue "User.StepStrength" (`KismetMathLibrary.SelectFloat` 1.4 1.0 bSprinting))
        (`ActorComponent.Activate` _returnvalue false)))))

(fn `UserConstructionScript`)